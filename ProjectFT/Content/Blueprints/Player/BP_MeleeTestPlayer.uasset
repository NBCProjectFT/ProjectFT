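; BP_MeleeTestPlayer is a test player Blueprint for damaging destructible store displays.
; On BeginPlay it creates a WBP_Progress widget and adds it to the viewport.
; Pressing G fires a short Visibility line trace forward from the follow camera and applies a small fixed damage to the hit actor.
; The trace has no actor-type filter, and the input is a hard-coded key event.
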(event EventBeginPlay
  (bind _returnvalue (UserInterface|CreateWidget "/Game/Blueprints/Player/Interaction/WBP_Progress.WBP_Progress_C"))
  (UserInterface|Viewport|AddtoViewport _returnvalue 0))

(event Collision|EventActorBeginOverlap
  (params (OtherActor :type Actor%20Object%20Reference)))

(event EventTick
  (params (DeltaSeconds :type Float%20%28single-precision%29)))

(event Input|KeyboardEvents|G
  (params (Key :type Key%20Structure :default "None"))
  (bind _followcamera (Variables|Default|GetFollowCamera))
  (bind _returnvalue (Transformation|GetWorldLocation _followcamera))
  ;[0.1029 0.15 0 0.5] 파괴형 매대 상호작용
  (:Pressed
    (bind (_outhit _returnvalue_2) (Collision|LineTraceByChannel _returnvalue (+ _returnvalue (* (Math|Vector|GetForwardVector _followcamera) 3e+02)) "TraceTypeQuery1" false 0 "None"))
    (if _returnvalue_2
      (Game|Damage|ApplyDamage (.HitActor (Collision|BreakHitResult _outhit)) 1e+01 0 0))))

(fn ConstructionScript)