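; BP_HubTempPlayerCharacter is a temporary hub player character for interacting with destructible stands and widgets.
; On BeginPlay it shows the progress widget, adds an AK47 to FTInventory and assigns it to a quick slot.
; G line-traces a short distance from the follow camera and applies damage to the hit actor.
; Left mouse forwards press and release to WidgetInteraction as pointer clicks, with debug prints.
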(event EventBeginPlay
  (bind _ftinventory (Variables|Default|GetFTInventory))
  (bind _returnvalue (UserInterface|CreateWidget "/Game/Blueprints/Player/Interaction/WBP_Progress.WBP_Progress_C"))
  (UserInterface|Viewport|AddtoViewport _returnvalue 0)
  (bind _returnvalue_2 (Class|FTInventoryComponent|AddItem _ftinventory "AK47" 1))
  (Class|FTInventoryComponent|SetQuickSlot _ftinventory 0 "AK47")
  (Development|PrintString (Utilities|String|ToString(Boolean) _returnvalue_2)))

(event Collision|EventActorBeginOverlap
  (params (OtherActor :type Actor%20Object%20Reference)))

(event EventTick
  (params (DeltaSeconds :type Float%20%28single-precision%29)))

(event Input|KeyboardEvents|G
  (params (Key :type Key%20Structure :default "None"))
  (bind _followcamera (Variables|Default|GetFollowCamera))
  (bind _returnvalue (Transformation|GetWorldLocation _followcamera))
  ;[0.1029 0.15 0 0.5] 파괴형 매대 상호작용
  (:Pressed
    (bind (_outhit _returnvalue_2) (Collision|LineTraceByChannel _returnvalue (+ _returnvalue (* (Math|Vector|GetForwardVector _followcamera) 3e+02)) "TraceTypeQuery1" false 0 "None"))
    (if _returnvalue_2
      (Game|Damage|ApplyDamage (.HitActor (Collision|BreakHitResult _outhit)) 1e+01 0 0))))

(event Input|MouseEvents|LeftMouseButton
  (params (Key :type Key%20Structure :default "None"))
  (:Pressed
    (Class|WidgetInteractionComponent|PressPointerKey (Variables|Default|GetWidgetInteraction) "LeftMouseButton")
    (Development|PrintString "눌림"))
  (:Released
    (Class|WidgetInteractionComponent|ReleasePointerKey (Variables|Default|GetWidgetInteraction) "LeftMouseButton")
    (Development|PrintString "Epwla")))

(fn ConstructionScript)