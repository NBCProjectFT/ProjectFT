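; GA_ForceGunScan is a gameplay ability that holds the avatar character in a rifle firing pose while the use input is held.
; On activation it plays a firing montage, then freezes it shortly after by setting its play rate to zero.
; When an Event.UseReleased gameplay event arrives, it resumes the montage and ends the ability after a short delay; montage interruption also ends it.
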(event Ability|EventActivateAbility
  (bind _ascharacter (Utilities|Casting|CastToCharacter (Ability|GetAvatarActorfromActorInfo)))
  (|PlayMontageandWaitProxy "None" "/Game/Assets/Characters/NekoRetarget/Anims/Armed/Firing_Rifle_Anim1_Montage_Neko.Firing_Rifle_Anim1_Montage_Neko" 1.0 "None" true 1.0 0.0 false
    (:then
      (Utilities|FlowControl|Delay 0.2)
      (Animation|Montage|MontageSetPlayRate (Components|SkeletalMesh|GetAnimInstance (Variables|/Script/Engine.Character|GetMesh _ascharacter)) "/Game/Assets/Characters/NekoRetarget/Anims/Armed/Firing_Rifle_Anim1_Montage_Neko.Firing_Rifle_Anim1_Montage_Neko" 0.0)
      (Ability|Tasks|WaitGameplayEvent "(TagName=\"Event.UseReleased\")" 0
        (:EventReceived
          (Animation|Montage|MontageSetPlayRate (Components|SkeletalMesh|GetAnimInstance (Variables|/Script/Engine.Character|GetMesh _ascharacter)) "/Game/Assets/Characters/NekoRetarget/Anims/Armed/Firing_Rifle_Anim1_Montage_Neko.Firing_Rifle_Anim1_Montage_Neko" 1.0)
          (Utilities|FlowControl|Delay 0.3)
          (Ability|EndAbility))))
    (:OnInterrupted
      (Ability|EndAbility))))